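; Player character Blueprint for a shooter, turning input actions into movement states, firing and reloading.
; Move and sprint inputs only set walking and running flags, with sprint requiring walking, while fire input calls Fire.
; Reload is guarded by a Reloading flag, calls Reload and plays paired MX16A4 montages, including a first-person one on SkeletalMesh, which GetTargetMesh returns.
; An older delay-based reload chain is left unconnected.
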(event `EnhancedInput|/Game/Input/MoveForward`
  (params (ActionValue :type "Vector2D Structure") (ElapsedSeconds :type "Float (double-precision)") (TriggeredSeconds :type "Float (double-precision)") (InputAction :type "InputAction Object Reference" :default "/Game/Input/MoveForward.MoveForward"))
  (:`Triggered`
    (set `self.bIsWalking` true))
  (:`Completed`
    (set `self.bIsWalking` false)))

(event `EnhancedInput|/Game/Input/SprintAction`
  (params (ActionValue :type Boolean) (ElapsedSeconds :type "Float (double-precision)") (TriggeredSeconds :type "Float (double-precision)") (InputAction :type "InputAction Object Reference" :default "/Game/Input/SprintAction.SprintAction"))
  (:`Triggered`
    (if (`self.bIsWalking`)
      (set `self.bIsRuning` true)))
  (:`Completed`
    (set `self.bIsRuning` false)))

(event `EnhancedInput|/Game/Input/MoveRight`
  (params (ActionValue :type "Vector2D Structure") (ElapsedSeconds :type "Float (double-precision)") (TriggeredSeconds :type "Float (double-precision)") (InputAction :type "InputAction Object Reference" :default "/Game/Input/MoveRight.MoveRight"))
  (:`Triggered`
    (set `self.bIsWalking` true))
  (:`Completed`
    (set `self.bIsWalking` false)))

(event `EnhancedInput|/Game/Input/Fire`
  (params (ActionValue :type Boolean) (ElapsedSeconds :type "Float (double-precision)") (TriggeredSeconds :type "Float (double-precision)") (InputAction :type "InputAction Object Reference" :default "/Game/Input/Fire.Fire"))
  (:`Triggered`
    (`self.Fire`)))

(event `EnhancedInput|/Game/Input/ReloadAction`
  (params (ActionValue :type Boolean) (ElapsedSeconds :type "Float (double-precision)") (TriggeredSeconds :type "Float (double-precision)") (InputAction :type "InputAction Object Reference" :default "/Game/Input/ReloadAction.ReloadAction"))
  (:`Started`
    (if (not (`self.reloading`))
      (set `self.reloading` true)
      (`self.Reload`)
      (`|PlayMontage` null "/Game/FPSAnimationPack/Animations/UE4/MX16A4/Weapon/AM_MX16A4_Reload_Tac.AM_MX16A4_Reload_Tac"
        (:`then`
          (`|PlayMontage` (`self.SkeletalMesh`) "/FPSAnimationPack/Animations/UE4/MX16A4/Character/AM_FP_MX16A4_Reload_Tac.AM_FP_MX16A4_Reload_Tac"))
        (:`OnCompleted`
          (set `self.reloading` false))))))

(event `EnhancedInput|/Game/Input/ReloadAction`
  (params (ActionValue :type Boolean) (ElapsedSeconds :type "Float (double-precision)") (TriggeredSeconds :type "Float (double-precision)") (InputAction :type "InputAction Object Reference" :default "/Game/Input/ReloadAction.ReloadAction")))

(fn `get target mesh`
  (returns (targetmesh :type "SkeletalMeshComponent Object Reference"))
  (return (`self.SkeletalMesh`)))

(fn `ReloadContorl`
  (`self.Reload`)
  (set `self.reloading` true))

(fn `UserConstructionScript`)