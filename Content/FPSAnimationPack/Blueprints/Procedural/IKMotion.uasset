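; IKMotion is a procedural animation asset in the FPS animation pack that defines a curve-driven motion offset.
; Evaluate samples the Position and Rotation vector curves at a given time, applies their scale multipliers, and outputs location, rotation and unit scale.
; Rotation curve X, Y and Z map to roll, pitch and yaw.
; GetLength reports the later end time of the two curves as the motion's duration.
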(fn `Evaluate`
  (params (Time :type "Float (double-precision)"))
  (returns (Motion :type "Transform Structure"))
  (bind (_returnvalue_x _returnvalue_y _returnvalue_z) (`KismetMathLibrary.BreakVector` (* (`CurveVector.GetVectorValue` (`self.Rotation`) Time) (`self.RotationScale`))))
  (return (`KismetMathLibrary.MakeTransform` (* (`CurveVector.GetVectorValue` (`self.Position`) Time) (`self.PositionScale`)) (`KismetMathLibrary.MakeRotator` _returnvalue_x _returnvalue_y _returnvalue_z))))

(fn `GetLength`
  (returns (Length :type "Float (double-precision)"))
  (return (`KismetMathLibrary.FMax` (`.MaxTime` (`CurveBase.GetTimeRange` (`self.Rotation`))) (`.MaxTime` (`CurveBase.GetTimeRange` (`self.Position`))))))