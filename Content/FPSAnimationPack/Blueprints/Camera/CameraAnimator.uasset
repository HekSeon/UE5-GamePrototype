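; Camera animation component for the viewmodel character that drives camera rotation and aim zoom.
; Each tick, after the owner ticks, it combines control rotation with CameraRoll, CameraPitch and CameraYaw animation curves and a recoil shake using quaternion multiplication.
; PlayRecoilShake randomizes per-axis amplitudes, then a vector curve scales them over time with interpolated smoothing.
; FOV eases sinusoidally between the base and aim values based on the ViewmodelController's aiming state.
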(event `self.ReceiveBeginPlay`
  (bind _asbp_viewmodel_character (cast `/Game/FPSAnimationPack/Blueprints/Character/BP_ViewmodelCharacter` (`self.GetOwner`)))
  (set `self.OwnerCharacter` _asbp_viewmodel_character)
  (set `self.Camera` (`Actor.GetComponentByClass` _asbp_viewmodel_character "/Script/Engine.CameraComponent"))
  (`self.AddTickPrerequisiteActor` (`self.GetOwner`))
  (set `self.BaseFOV` (`CameraComponent.FieldOfView` (`self.Camera`))))

(event `self.ReceiveTick`
  (params (DeltaSeconds :type "Float (single-precision)"))
  (bind (_camerarecoilshake_x _camerarecoilshake_y _camerarecoilshake_z) (`KismetMathLibrary.BreakVector` (`self.CameraRecoilShake`)))
  (bind _mesh (`Character.Mesh` (`self.OwnerCharacter`)))
  (bind _returnvalue (`SkeletalMeshComponent.GetAnimInstance` _mesh))
  (`/Engine/EditorBlueprintResources/StandardMacros.IsValid` _mesh
    (:`Is Valid`
      (`/Engine/EditorBlueprintResources/StandardMacros.IsValid` _returnvalue
        (:`Is Valid`
          (`self.UpdateCameraShake`)
          (`SceneComponent.K2_SetWorldRotation` (`self.Camera`) (`KismetMathLibrary.Quat_Rotator` (* (`KismetMathLibrary.Conv_RotatorToQuaternion` (`Pawn.GetControlRotation` (`self.OwnerCharacter`))) (* (`KismetMathLibrary.Conv_RotatorToQuaternion` (`KismetMathLibrary.MakeRotator` (`AnimInstance.GetCurveValue` _returnvalue "CameraRoll") (`AnimInstance.GetCurveValue` _returnvalue "CameraPitch") (`AnimInstance.GetCurveValue` _returnvalue "CameraYaw"))) (`KismetMathLibrary.Conv_RotatorToQuaternion` (`KismetMathLibrary.MakeRotator` _camerarecoilshake_x _camerarecoilshake_y _camerarecoilshake_z))))) false false)
          (`self.UpdateFOV`))))))

(fn `PlayRecoilShake`
  (params (NewShake :type "/Game/FPSAnimationPack/Blueprints/Camera/CameraRecoilShake Object Reference"))
  (bind _activerecoilshake (`self.ActiveRecoilShake`))
  (bind (_pitch_x _pitch_y) (`KismetMathLibrary.BreakVector2D` (`/Game/FPSAnimationPack/Blueprints/Camera/CameraRecoilShake.Pitch` _activerecoilshake)))
  (bind (_yaw_x _yaw_y) (`KismetMathLibrary.BreakVector2D` (`/Game/FPSAnimationPack/Blueprints/Camera/CameraRecoilShake.Yaw` _activerecoilshake)))
  (bind (_roll_x _roll_y) (`KismetMathLibrary.BreakVector2D` (`/Game/FPSAnimationPack/Blueprints/Camera/CameraRecoilShake.Roll` _activerecoilshake)))
  (set `self.ActiveRecoilShake` NewShake)
  (set `self.IsShakePlaying` true)
  (set `self.ShakePlayback` 0.0)
  (set `self.ShakeTarget` (`KismetMathLibrary.MakeVector` (`KismetMathLibrary.RandomFloatInRange` _roll_x _roll_y) (`KismetMathLibrary.RandomFloatInRange` _pitch_x _pitch_y) (`KismetMathLibrary.RandomFloatInRange` _yaw_x _yaw_y))))

(fn `UpdateCameraShake`
  (if (`self.IsShakePlaying`)
    (`self.ActiveRecoilShake`
      (:`then`
        (set `self.CameraRecoilShake` (`KismetMathLibrary.VInterpTo` (`self.CameraRecoilShake`) (* (`CurveVector.GetVectorValue` (`/Game/FPSAnimationPack/Blueprints/Camera/CameraRecoilShake.RotationCurve` (`self.ActiveRecoilShake`)) (`self.ShakePlayback`)) (`self.ShakeTarget`)) (`GameplayStatics.GetWorldDeltaSeconds`) (`/Game/FPSAnimationPack/Blueprints/Camera/CameraRecoilShake.Smoothing` (`self.ActiveRecoilShake`))))
        (set `self.ShakePlayback` (+ (* (`GameplayStatics.GetWorldDeltaSeconds`) (`/Game/FPSAnimationPack/Blueprints/Camera/CameraRecoilShake.PlayRate` (`self.ActiveRecoilShake`))) (`self.ShakePlayback`)))
        (if (>= (`self.ShakePlayback`) (`.MaxTime` (`CurveBase.GetTimeRange` (`/Game/FPSAnimationPack/Blueprints/Camera/CameraRecoilShake.RotationCurve` (`self.ActiveRecoilShake`)))))
          (set `self.IsShakePlaying` false)))
      (:`else`))))

(fn `UpdateFOV`
  (set `self.AimingPlayback` (`KismetMathLibrary.FClamp` (+ (* (`KismetMathLibrary.SelectFloat` 1.0 -1.0 (`/Game/FPSAnimationPack/Blueprints/Character/ViewmodelController.IsAiming` (`/Game/FPSAnimationPack/Blueprints/Character/BP_ViewmodelCharacter.ViewmodelController` (`self.OwnerCharacter`)))) (`GameplayStatics.GetWorldDeltaSeconds`) (`self.AimingSpeed`)) (`self.AimingPlayback`))))
  (`CameraComponent.SetFieldOfView` (`self.Camera`) (`|EaseFunction` "SinusoidalInOut" (`self.AimingPlayback`) (`self.BaseFOV`) (`self.AimFOV`))))