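; Base first-person weapon actor for a BP_ViewmodelCharacter, handling firing, reloading, fire modes, interact and grenade-throw animations from a weapon settings asset.
; Equipping binds the character's input events and initializes its recoil component; unequipping unbinds them.
; Fire drives ammo, camera shake, recoil, sound and paired character/weapon montages, re-calling itself by delay in Auto.
; Reload picks empty or non-empty montages and refills ammo on a timer scaled from montage length.
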(event `Initialize`
  (params (Settings :type "/Game/FPSAnimationPack/Blueprints/Character/WeaponSettings Object Reference"))
  (bind _output_get (set `self.WeaponSettings` Settings))
  (set `self.Ammo` (`/Game/FPSAnimationPack/Blueprints/Character/WeaponSettings.Ammo` _output_get))
  (set `self.ViewmodelSettings` (`/Game/FPSAnimationPack/Blueprints/Character/WeaponSettings.UE4` (`self.WeaponSettings`)))
  (bind _asbp_viewmodel_character (cast `/Game/FPSAnimationPack/Blueprints/Character/BP_ViewmodelCharacter` (`self.GetOwner`)))
  (set `self.OwnerCharacter` _asbp_viewmodel_character))

(event `Fire`
  (bind _ownercharacter (`self.OwnerCharacter`))
  (bind (_weaponanims_primaryreload _weaponanims_secondaryreload _weaponanims_additionalreload _weaponanims_equip _weaponanims_unequip _weaponanims_action _weaponanims_fire _weaponanims_fireout) (break `/Game/FPSAnimationPack/Blueprints/Character/F_ViewmodelAnimations` (`/Game/FPSAnimationPack/Blueprints/Character/WeaponSettings.WeaponAnims` (`self.WeaponSettings`))))
  (bind (_characteranims_primaryreload _characteranims_secondaryreload _characteranims_additionalreload _characteranims_equip _characteranims_unequip _characteranims_action _characteranims_fire) (break `/Game/FPSAnimationPack/Blueprints/Character/F_ViewmodelAnimations` (`/Game/FPSAnimationPack/Blueprints/Character/ViewmodelSettings.CharacterAnims` (`self.ViewmodelSettings`))))
  (if (`self.IsFiring`)
    (if (> (`self.Ammo`) 0)
      (`KismetSystemLibrary.K2_ClearAndInvalidateTimerHandle` (`self.FireTimer`))
      (set `self.Ammo` (- (`self.Ammo`) 1))
      (`/Game/FPSAnimationPack/Blueprints/Camera/CameraAnimator.PlayRecoilShake` (`/Game/FPSAnimationPack/Blueprints/Character/BP_ViewmodelCharacter.CameraAnimator` (`self.OwnerCharacter`)) (`/Game/FPSAnimationPack/Blueprints/Character/WeaponSettings.RecoilShake` (`self.WeaponSettings`)))
      (`RecoilAnimationComponent.Play` (`/Game/FPSAnimationPack/Blueprints/Character/BP_ViewmodelCharacter.RecoilAnimation` (`self.OwnerCharacter`)))
      (`GameplayStatics.PlaySoundAtLocation` (`/Game/FPSAnimationPack/Blueprints/Character/WeaponSettings.FireSound` (`self.WeaponSettings`)) (`SceneComponent.K2_GetComponentLocation` (`/Game/FPSAnimationPack/Blueprints/Character/BP_ViewmodelCharacter.WeaponMesh` (`self.OwnerCharacter`))) (struct) 1.0 1.0 0.0 null null null null)
      (`Character.PlayAnimMontage` _ownercharacter _characteranims_fire 1.0 "None")
      (`|PlayMontage` (`/Game/FPSAnimationPack/Blueprints/Character/BP_ViewmodelCharacter.WeaponMesh` _ownercharacter) (select `bool` (and (`KismetSystemLibrary.IsValid` _weaponanims_fireout) (== (`self.Ammo`) 0)) :`false` _weaponanims_fire :`true` _weaponanims_fireout)
        (:`then`
          (if (`|EnumEquality` (`self.FireMode`) "Auto")
            (if (== (`self.Ammo`) 0)
              (`self.StopFiring`))
            (`KismetSystemLibrary.Delay` (/ 60.0 (`/Game/FPSAnimationPack/Blueprints/Character/WeaponSettings.FireRate` (`self.WeaponSettings`))))
            (`self.Fire`)
            (else
              (bind _returnvalue (`KismetSystemLibrary.K2_SetTimerDelegate` (`|CreateDelegate` :!event `StopFiring`) 0.1))
              (set `self.FireTimer` _returnvalue))))))))

(event `Grenade`
  (bind _returnvalue (`Character.PlayAnimMontage` (`self.OwnerCharacter`) (`.UnEquip_14_A422DF6C40257AAAC8926E9B23DFAA41` (break `/Game/FPSAnimationPack/Blueprints/Character/F_ViewmodelAnimations` (`/Game/FPSAnimationPack/Blueprints/Character/ViewmodelSettings.CharacterAnims` (`self.ViewmodelSettings`)))) 1.0 "None"))
  (`KismetSystemLibrary.Delay` _returnvalue)
  (`SceneComponent.SetVisibility` (`/Game/FPSAnimationPack/Blueprints/Character/BP_ViewmodelCharacter.WeaponMesh` (`self.OwnerCharacter`)) false true)
  (bind _returnvalue_2 (`Character.PlayAnimMontage` (`self.OwnerCharacter`) (`.Action_17_103672494DED39772B314E9EAD265FD3` (break `/Game/FPSAnimationPack/Blueprints/Character/F_ViewmodelAnimations` (`/Game/FPSAnimationPack/Blueprints/Character/ViewmodelSettings.CharacterAnims` (`self.ViewmodelSettings`)))) 1.0 "None"))
  (`KismetSystemLibrary.Delay` (* _returnvalue_2 0.9))
  (bind _returnvalue_3 (`Character.PlayAnimMontage` (`self.OwnerCharacter`) (`.Equip_12_E991548C4D5C0EBB16A7DFA9E6241BB7` (break `/Game/FPSAnimationPack/Blueprints/Character/F_ViewmodelAnimations` (`/Game/FPSAnimationPack/Blueprints/Character/ViewmodelSettings.CharacterAnims` (`self.ViewmodelSettings`)))) 1.0 "None"))
  (`KismetSystemLibrary.Delay` (* _returnvalue_3 0.2))
  (`SceneComponent.SetVisibility` (`/Game/FPSAnimationPack/Blueprints/Character/BP_ViewmodelCharacter.WeaponMesh` (`self.OwnerCharacter`)) true true))

(fn `ChangeFireMode`
  (locals (PrevFireMode :type "EFireMode_PRAS Enum"))
  (bind _firemode (`/Game/FPSAnimationPack/Blueprints/Character/WeaponSettings.FireMode` (`self.WeaponSettings`)))
  (set `local.PrevFireMode` (`self.FireMode`))
  (`|ExecutionSequence`
    (:`then_0`
      (switch `EFireMode_PRAS` (`self.FireMode`)
        (:`Semi`
          (if (`KismetArrayLibrary.Array_Contains` _firemode "Burst")
            (set `self.FireMode` "Burst")
            (else
              (if (`KismetArrayLibrary.Array_Contains` _firemode "Auto") :!label _label
                (set `self.FireMode` "Auto")
                (else
                  (set `self.FireMode` "Semi"))))))
        (:`Auto`
          (set `self.FireMode` "Semi"))
        (:`Burst`
          (goto _label))))
    (:`then_1`
      (`RecoilAnimationComponent.SetFireMode` (`/Game/FPSAnimationPack/Blueprints/Character/BP_ViewmodelCharacter.RecoilAnimation` (`self.OwnerCharacter`)) (`self.FireMode`))
      (if (`|EnumInequality` (`self.FireMode`) (`local.PrevFireMode`))
        (`/Game/FPSAnimationPack/Blueprints/Character/ViewmodelController.PlayIKMotion` (`/Game/FPSAnimationPack/Blueprints/Character/BP_ViewmodelCharacter.ViewmodelController` (`self.OwnerCharacter`)) "/Game/FPSAnimationPack/Blueprints/Procedural/Ads/IK_FireMode.IK_FireMode")
        (`GameplayStatics.PlaySound2D` "/Game/FPSAnimationPack/SFX/General/S_FireMode.S_FireMode" (`KismetMathLibrary.RandomFloatInRange` 0.33 0.36) (`KismetMathLibrary.RandomFloatInRange` 1.05 1.07) 0.0 null null)))))

(fn `Interact`
  (bind (_characteranims_primaryreload _characteranims_secondaryreload _characteranims_additionalreload _characteranims_equip _characteranims_unequip _characteranims_action) (break `/Game/FPSAnimationPack/Blueprints/Character/F_ViewmodelAnimations` (`/Game/FPSAnimationPack/Blueprints/Character/ViewmodelSettings.CharacterAnims` (`self.ViewmodelSettings`))))
  (`Character.PlayAnimMontage` (`self.OwnerCharacter`) _characteranims_action 1.0 "None"))

(fn `OnEquipped`
  (bind _weaponsettings (`self.WeaponSettings`))
  (bind (_weaponanims_primaryreload _weaponanims_secondaryreload _weaponanims_additionalreload _weaponanims_equip _weaponanims_unequip _weaponanims_action _weaponanims_fire _weaponanims_fireout) (break `/Game/FPSAnimationPack/Blueprints/Character/F_ViewmodelAnimations` (`/Game/FPSAnimationPack/Blueprints/Character/WeaponSettings.WeaponAnims` (`self.WeaponSettings`))))
  (bind _recoilanimation (`/Game/FPSAnimationPack/Blueprints/Character/BP_ViewmodelCharacter.RecoilAnimation` (`self.OwnerCharacter`)))
  (bind (_returnvalue_location _returnvalue_rotation _returnvalue_scale) (`KismetMathLibrary.BreakTransform` (`SceneComponent.GetSocketTransform` (`/Game/FPSAnimationPack/Blueprints/Character/BP_ViewmodelCharacter.WeaponMesh` (`self.OwnerCharacter`)) "AimPoint" "RTS_Component")))
  (add `/Game/FPSAnimationPack/Blueprints/Character/BP_ViewmodelCharacter.OnReloadPressed` (`self.OwnerCharacter`) (`|CreateDelegate` :!event `ReloadWeapon`))
  (add `/Game/FPSAnimationPack/Blueprints/Character/BP_ViewmodelCharacter.OnFirePressed` (`self.OwnerCharacter`) (`|CreateDelegate` :!event `StartFiring`))
  (add `/Game/FPSAnimationPack/Blueprints/Character/BP_ViewmodelCharacter.OnFireReleased` (`self.OwnerCharacter`) (`|CreateDelegate` :!event `StopFiring`))
  (add `/Game/FPSAnimationPack/Blueprints/Character/BP_ViewmodelCharacter.OnInteractPressed` (`self.OwnerCharacter`) (`|CreateDelegate` :!event `Interact`))
  (add `/Game/FPSAnimationPack/Blueprints/Character/BP_ViewmodelCharacter.OnFireMode` (`self.OwnerCharacter`) (`|CreateDelegate` :!event `ChangeFireMode`))
  (add `/Game/FPSAnimationPack/Blueprints/Character/BP_ViewmodelCharacter.OnGrenade` (`self.OwnerCharacter`) (`|CreateDelegate` :!event `ThrowGrenade`))
  (`self.SetActorTickEnabled` true)
  (`RecoilAnimationComponent.SetFireMode` _recoilanimation (`self.FireMode`))
  (`RecoilAnimationComponent.Init` _recoilanimation (`/Game/FPSAnimationPack/Blueprints/Character/WeaponSettings.RecoilSettings` _weaponsettings) (`/Game/FPSAnimationPack/Blueprints/Character/WeaponSettings.FireRate` _weaponsettings) 0)
  (set `self.AimPoint` (`KismetMathLibrary.MakeTransform` (* _returnvalue_location -1.0) _returnvalue_rotation _returnvalue_scale))
  (if (== (`self.Ammo`) 0)
    (`AnimInstance.Montage_Play` (`SkeletalMeshComponent.GetAnimInstance` (`/Game/FPSAnimationPack/Blueprints/Character/BP_ViewmodelCharacter.WeaponMesh` (`self.OwnerCharacter`))) _weaponanims_fireout 1.0 "MontageLength" (* (`AnimationAsset.GetPlayLength` _weaponanims_fireout) 0.95) true)))

(fn `OnReloadEnded`
  (set `self.Ammo` (`/Game/FPSAnimationPack/Blueprints/Character/WeaponSettings.Ammo` (`self.WeaponSettings`))))

(fn `OnUnEquipped`
  (clear `/Game/FPSAnimationPack/Blueprints/Character/BP_ViewmodelCharacter.OnReloadPressed` (`self.OwnerCharacter`))
  (clear `/Game/FPSAnimationPack/Blueprints/Character/BP_ViewmodelCharacter.OnFirePressed` (`self.OwnerCharacter`))
  (clear `/Game/FPSAnimationPack/Blueprints/Character/BP_ViewmodelCharacter.OnFireReleased` (`self.OwnerCharacter`))
  (clear `/Game/FPSAnimationPack/Blueprints/Character/BP_ViewmodelCharacter.OnInteractPressed` (`self.OwnerCharacter`))
  (clear `/Game/FPSAnimationPack/Blueprints/Character/BP_ViewmodelCharacter.OnFireMode` (`self.OwnerCharacter`))
  (clear `/Game/FPSAnimationPack/Blueprints/Character/BP_ViewmodelCharacter.OnGrenade` (`self.OwnerCharacter`))
  (`self.SetActorTickEnabled` false))

(fn `ReloadWeapon`
  (bind _returnvalue (== (`self.Ammo`) 0))
  (bind (_characteranims_primaryreload _characteranims_secondaryreload) (break `/Game/FPSAnimationPack/Blueprints/Character/F_ViewmodelAnimations` (`/Game/FPSAnimationPack/Blueprints/Character/ViewmodelSettings.CharacterAnims` (`self.ViewmodelSettings`))))
  (bind (_weaponanims_primaryreload _weaponanims_secondaryreload) (break `/Game/FPSAnimationPack/Blueprints/Character/F_ViewmodelAnimations` (`/Game/FPSAnimationPack/Blueprints/Character/WeaponSettings.WeaponAnims` (`self.WeaponSettings`))))
  (if (< (`self.Ammo`) (`/Game/FPSAnimationPack/Blueprints/Character/WeaponSettings.Ammo` (`self.WeaponSettings`)))
    (`Character.PlayAnimMontage` (`self.OwnerCharacter`) (select `bool` _returnvalue :`false` _characteranims_secondaryreload :`true` _characteranims_primaryreload) 1.0 "None")
    (bind _returnvalue_2 (`AnimInstance.Montage_Play` (`SkeletalMeshComponent.GetAnimInstance` (`/Game/FPSAnimationPack/Blueprints/Character/BP_ViewmodelCharacter.WeaponMesh` (`self.OwnerCharacter`))) (select `bool` _returnvalue :`false` _weaponanims_secondaryreload :`true` _weaponanims_primaryreload) 1.0 "MontageLength" 0.0 true))
    (`KismetSystemLibrary.K2_SetTimerDelegate` (`|CreateDelegate` :!event `OnReloadEnded`) (* _returnvalue_2 (`/Game/FPSAnimationPack/Blueprints/Character/WeaponSettings.AmmoRefilTimeScale` (`self.WeaponSettings`))))))

(fn `StartFiring`
  (if (>= (- (`KismetSystemLibrary.GetGameTimeInSeconds`) (`self.LastFireTime`)) (/ 60.0 (`/Game/FPSAnimationPack/Blueprints/Character/WeaponSettings.FireRate` (`self.WeaponSettings`))))
    (set `self.IsFiring` true)
    (set `self.LastFireTime` (`KismetSystemLibrary.GetGameTimeInSeconds`))
    (`self.Fire`)))

(fn `StopFiring`
  (set `self.IsFiring` false)
  (`RecoilAnimationComponent.Stop` (`/Game/FPSAnimationPack/Blueprints/Character/BP_ViewmodelCharacter.RecoilAnimation` (`self.OwnerCharacter`))))

(fn `ThrowGrenade`
  (`self.Grenade`))

(fn `UserConstructionScript`)