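; Weapon Blueprint for manual-action guns in an FPS animation pack, reloading one cartridge at a time.
; ReloadWeapon plays the primary reload montages on character and weapon mesh when ammo is below capacity, setting a timer for the montage length.
; InsertCartrdige plays secondary montages, waits out the animation, increments Ammo, then calls itself again until capacity is reached, finishing with the additional reload montages.
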(event `InsertCartrdige`
  (`AnimInstance.Montage_Play` (`SkeletalMeshComponent.GetAnimInstance` (`/Game/FPSAnimationPack/Blueprints/Character/BP_ViewmodelCharacter.WeaponMesh` (`self.OwnerCharacter`))) (`.SecondaryReload_23_AA7999D74A8CAAFDE00E34A800A2CACF` (break `/Game/FPSAnimationPack/Blueprints/Character/F_ViewmodelAnimations` (`/Game/FPSAnimationPack/Blueprints/Character/WeaponSettings.WeaponAnims` (`self.WeaponSettings`)))) 1.0 "MontageLength" 0.0 true)
  (bind _returnvalue (`Character.PlayAnimMontage` (`self.OwnerCharacter`) (`.SecondaryReload_23_AA7999D74A8CAAFDE00E34A800A2CACF` (break `/Game/FPSAnimationPack/Blueprints/Character/F_ViewmodelAnimations` (`/Game/FPSAnimationPack/Blueprints/Character/ViewmodelSettings.CharacterAnims` (`self.ViewmodelSettings`)))) 1.0 "None"))
  (`KismetSystemLibrary.Delay` _returnvalue)
  (`/Engine/EditorBlueprintResources/StandardMacros.IncrementInt` (`self.Ammo`)
    (:`  `
      (if (== (`self.Ammo`) (`/Game/FPSAnimationPack/Blueprints/Character/WeaponSettings.Ammo` (`self.WeaponSettings`)))
        (`Character.PlayAnimMontage` (`self.OwnerCharacter`) (`.AdditionalReload_26_8CD73B38491EE72B09315E85F1BEBC5B` (break `/Game/FPSAnimationPack/Blueprints/Character/F_ViewmodelAnimations` (`/Game/FPSAnimationPack/Blueprints/Character/ViewmodelSettings.CharacterAnims` (`self.ViewmodelSettings`)))) 1.0 "None")
        (`AnimInstance.Montage_Play` (`SkeletalMeshComponent.GetAnimInstance` (`/Game/FPSAnimationPack/Blueprints/Character/BP_ViewmodelCharacter.WeaponMesh` (`self.OwnerCharacter`))) (`.AdditionalReload_26_8CD73B38491EE72B09315E85F1BEBC5B` (break `/Game/FPSAnimationPack/Blueprints/Character/F_ViewmodelAnimations` (`/Game/FPSAnimationPack/Blueprints/Character/WeaponSettings.WeaponAnims` (`self.WeaponSettings`)))) 1.0 "MontageLength" 0.0 true)
        (else
          (`self.InsertCartrdige`))))))

(fn `ReloadWeapon`
  (if (< (`self.Ammo`) (`/Game/FPSAnimationPack/Blueprints/Character/WeaponSettings.Ammo` (`self.WeaponSettings`)))
    (bind _returnvalue (`Character.PlayAnimMontage` (`self.OwnerCharacter`) (`.PrimaryReload_22_357D3BE24A5668E479824EB13B542904` (break `/Game/FPSAnimationPack/Blueprints/Character/F_ViewmodelAnimations` (`/Game/FPSAnimationPack/Blueprints/Character/ViewmodelSettings.CharacterAnims` (`self.ViewmodelSettings`)))) 1.0 "Default"))
    (`KismetSystemLibrary.K2_SetTimerDelegate` (`|CreateDelegate` :!event `InsertCartrdige`) _returnvalue)
    (`AnimInstance.Montage_Play` (`SkeletalMeshComponent.GetAnimInstance` (`/Game/FPSAnimationPack/Blueprints/Character/BP_ViewmodelCharacter.WeaponMesh` (`self.OwnerCharacter`))) (`.PrimaryReload_22_357D3BE24A5668E479824EB13B542904` (break `/Game/FPSAnimationPack/Blueprints/Character/F_ViewmodelAnimations` (`/Game/FPSAnimationPack/Blueprints/Character/WeaponSettings.WeaponAnims` (`self.WeaponSettings`)))) 1.0 "MontageLength" 0.0 true)))

(fn `UserConstructionScript`
  (`parent.UserConstructionScript`))