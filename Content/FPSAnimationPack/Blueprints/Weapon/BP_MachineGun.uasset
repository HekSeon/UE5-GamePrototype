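; BP_MachineGun is the machine gun weapon Blueprint, defining its reload behavior and little else.
; ReloadWeapon runs only when ammo is below capacity, choosing among three reload animations: empty, above a hardcoded round threshold, or in between.
; It plays matching montages on the owning character and its weapon mesh, using settings structs for the assets.
; The weapon montage's length, scaled by AmmoRefilTimeScale, sets a timer for a follow-up event.
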(fn `ReloadWeapon`
  (bind ((`PrimaryReload_22_357D3BE24A5668E479824EB13B542904` _primaryreload) (`SecondaryReload_23_AA7999D74A8CAAFDE00E34A800A2CACF` _secondaryreload) (`AdditionalReload_26_8CD73B38491EE72B09315E85F1BEBC5B` _additionalreload)) (break `/Game/FPSAnimationPack/Blueprints/Character/F_ViewmodelAnimations` (`/Game/FPSAnimationPack/Blueprints/Character/WeaponSettings.WeaponAnims` (`self.WeaponSettings`))))
  (bind ((`PrimaryReload_22_357D3BE24A5668E479824EB13B542904` _primaryreload_2) (`SecondaryReload_23_AA7999D74A8CAAFDE00E34A800A2CACF` _secondaryreload_2) (`AdditionalReload_26_8CD73B38491EE72B09315E85F1BEBC5B` _additionalreload_2)) (break `/Game/FPSAnimationPack/Blueprints/Character/F_ViewmodelAnimations` (`/Game/FPSAnimationPack/Blueprints/Character/ViewmodelSettings.CharacterAnims` (`self.ViewmodelSettings`))))
  (if (< (`self.Ammo`) (`/Game/FPSAnimationPack/Blueprints/Character/WeaponSettings.Ammo` (`self.WeaponSettings`)))
    (`Character.PlayAnimMontage` (`self.OwnerCharacter`) (select `bool` (== (`self.Ammo`) 0) :`false` (select `bool` (> (`self.Ammo`) 22) :`false` _additionalreload_2 :`true` _secondaryreload_2) :`true` _primaryreload_2) 1.0 "None")
    (bind _returnvalue (`AnimInstance.Montage_Play` (`SkeletalMeshComponent.GetAnimInstance` (`/Game/FPSAnimationPack/Blueprints/Character/BP_ViewmodelCharacter.WeaponMesh` (`self.OwnerCharacter`))) (select `bool` (== (`self.Ammo`) 0) :`false` (select `bool` (> (`self.Ammo`) 22) :`false` _additionalreload :`true` _secondaryreload) :`true` _primaryreload) 1.0 "MontageLength" 0.0 true))
    (`KismetSystemLibrary.K2_SetTimerDelegate` (`|CreateDelegate` :!event `OnReloadEnded`) (* _returnvalue (`/Game/FPSAnimationPack/Blueprints/Character/WeaponSettings.AmmoRefilTimeScale` (`self.WeaponSettings`))))))

(fn `UserConstructionScript`
  (`parent.UserConstructionScript`))