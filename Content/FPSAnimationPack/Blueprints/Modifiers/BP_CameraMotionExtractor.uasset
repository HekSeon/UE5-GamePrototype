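; Animation modifier that bakes camera bone rotation from a camera animation into float curves on the sequence it is applied to.
; On apply, it adds the named curves and caches the bone's local rotation from a reference animation.
; It then samples the camera animation at 30 fps, keying the Intensity-scaled rotation delta from that reference as negated roll, yaw and pitch.
; Reverting removes the curves.
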(event `self.OnApply`
  (params (AnimationSequence :type "AnimSequence Object Reference"))
  (set `self.Playback` 0.0)
  (`self.AddCurves` AnimationSequence)
  (while (< (`self.Playback`) (`AnimationBlueprintLibrary.GetSequenceLength` (`self.CameraAnimation`)))
    (bind _pose (`AnimPoseExtensions.GetAnimPoseAtTime` (`self.CameraAnimation`) (`self.Playback`) (make `AnimPoseEvaluationOptions` "Source" false)))
    (`|ExecutionSequence`
      (:`then_0`
        (bind (_returnvalue_location _returnvalue_rotation) (`KismetMathLibrary.BreakTransform` (`AnimPoseExtensions.GetBonePose` _pose (`self.CameraBoneName`))))
        (`self.AddCurveKeys` AnimationSequence (`self.Playback`) _returnvalue_rotation))
      (:`then_1`
        (set `self.Playback` (+ (`self.Playback`) (/ 1.0 30.0)))))))

(event `self.OnRevert`
  (params (AnimationSequence :type "AnimSequence Object Reference"))
  (`self.RemoveCurves` AnimationSequence))

(fn `AddCurveKeys`
  (params (Sequence :type "AnimSequence Object Reference") (Time :type "Float (double-precision)") (Value :type "Rotator Structure"))
  (bind _intensity (`self.Intensity`))
  (bind (_returnvalue_roll _returnvalue_pitch _returnvalue_yaw) (`KismetMathLibrary.BreakRotator` (`KismetMathLibrary.NormalizedDeltaRotator` Value (`self.RefPose`))))
  (`AnimationBlueprintLibrary.AddFloatCurveKey` Sequence (`|GetArrayItem` (`self.CurveNames`)) Time (* _intensity (* _returnvalue_roll -1.0)))
  (`AnimationBlueprintLibrary.AddFloatCurveKey` Sequence (`|GetArrayItem` (`self.CurveNames`) 1) Time (* _intensity _returnvalue_yaw))
  (`AnimationBlueprintLibrary.AddFloatCurveKey` Sequence (`|GetArrayItem` (`self.CurveNames`) 2) Time (* _intensity _returnvalue_pitch)))

(fn `AddCurves`
  (params (Sequence :type "AnimSequence Object Reference"))
  (for _array_element (`self.CurveNames`)
    (`AnimationBlueprintLibrary.AddCurve` Sequence _array_element))
  (bind _pose (`AnimPoseExtensions.GetAnimPoseAtFrame` (`self.RefAnimation`) 0 (make `AnimPoseEvaluationOptions` "Source" false)))
  (bind (_returnvalue_location _returnvalue_rotation) (`KismetMathLibrary.BreakTransform` (`AnimPoseExtensions.GetBonePose` _pose (`self.CameraBoneName`))))
  (set `self.RefPose` _returnvalue_rotation))

(fn `RemoveCurves`
  (params (Sequence :type "AnimSequence Object Reference"))
  (for _array_element (`self.CurveNames`)
    (`AnimationBlueprintLibrary.RemoveCurve` Sequence _array_element)))