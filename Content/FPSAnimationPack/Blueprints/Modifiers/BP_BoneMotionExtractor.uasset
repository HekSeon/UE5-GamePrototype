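; Animation modifier that bakes one bone's motion into six float curves for location and rotation, named from a shared prefix.
; On apply it samples the sequence at SampleRate and keys the bone's world-space pose relative to a reference pose.
; That reference is frame zero of SourceAnimation, defaulting to the sequence itself, using RefBoneName or the same bone.
; Sampling is nested inside the curve-creation loop, and revert removes the curves.
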(event `self.OnApply`
  (params (AnimationSequence :type "AnimSequence Object Reference"))
  (bind _animposeevaluationoptions (make `AnimPoseEvaluationOptions` "Source" false))
  (bind _refbonename (`self.RefBoneName`))
  (for _array_element (`self.CurveNames`)
    (`AnimationBlueprintLibrary.AddCurve` AnimationSequence (`KismetStringLibrary.Conv_StringToName` (`KismetStringLibrary.Concat_StrStr` (`KismetStringLibrary.Conv_NameToString` (`self.CurveName`)) (`KismetStringLibrary.Conv_NameToString` _array_element))))
    (`/Engine/EditorBlueprintResources/StandardMacros.IsValid` (`self.SourceAnimation`)
      (:`Is Valid`
        (`|ExecutionSequence`
          (:`then_0`
            (bind _pose (`AnimPoseExtensions.GetAnimPoseAtTime` (`self.SourceAnimation`) 0.0 _animposeevaluationoptions))
            (set `self.RefPose` (`AnimPoseExtensions.GetBonePose` _pose (select `bool` (== _refbonename "None") :`false` _refbonename :`true` (`self.BoneName`)) "World")))
          (:`then_1`
            (while (< (`self.Playback`) (`AnimationAsset.GetPlayLength` AnimationSequence))
              (bind _pose_2 (`AnimPoseExtensions.GetAnimPoseAtTime` AnimationSequence (`self.Playback`) _animposeevaluationoptions))
              (`self.AddTransformKey` AnimationSequence (`KismetMathLibrary.MakeRelativeTransform` (`AnimPoseExtensions.GetBonePose` _pose_2 (`self.BoneName`) "World") (`self.RefPose`)) (`self.Playback`))
              (set `self.Playback` (+ (`self.Playback`) (/ 1.0 (`self.SampleRate`)))))
            (set `self.Playback` 0.0))))
      (:`Is Not Valid`
        (set `self.SourceAnimation` AnimationSequence)))))

(event `self.OnRevert`
  (params (AnimationSequence :type "AnimSequence Object Reference"))
  (for _array_element (`self.CurveNames`)
    (`AnimationBlueprintLibrary.RemoveCurve` AnimationSequence (`KismetStringLibrary.Conv_StringToName` (`KismetStringLibrary.Concat_StrStr` (`KismetStringLibrary.Conv_NameToString` (`self.CurveName`)) (`KismetStringLibrary.Conv_NameToString` _array_element))))))

(fn `AddTransformKey`
  (params (Sequence :type "AnimSequence Object Reference") (Transform :type "Transform Structure") (Time :type "Float (double-precision)"))
  (bind _curvenames (`self.CurveNames`))
  (bind _curvenames_2 (`self.CurveNames`))
  (bind _returnvalue (`KismetStringLibrary.Conv_NameToString` (`self.CurveName`)))
  (bind _returnvalue_2 (`KismetStringLibrary.Conv_NameToString` (`self.CurveName`)))
  (`AnimationBlueprintLibrary.AddFloatCurveKey` Sequence (`KismetStringLibrary.Conv_StringToName` (`KismetStringLibrary.Concat_StrStr` _returnvalue (`KismetStringLibrary.Conv_NameToString` (`|GetArrayItem` _curvenames_2)))) Time (.x (.location Transform)))
  (`AnimationBlueprintLibrary.AddFloatCurveKey` Sequence (`KismetStringLibrary.Conv_StringToName` (`KismetStringLibrary.Concat_StrStr` _returnvalue (`KismetStringLibrary.Conv_NameToString` (`|GetArrayItem` _curvenames_2 1)))) Time (.y (.location Transform)))
  (`AnimationBlueprintLibrary.AddFloatCurveKey` Sequence (`KismetStringLibrary.Conv_StringToName` (`KismetStringLibrary.Concat_StrStr` _returnvalue (`KismetStringLibrary.Conv_NameToString` (`|GetArrayItem` _curvenames_2 2)))) Time (.z (.location Transform)))
  (`AnimationBlueprintLibrary.AddFloatCurveKey` Sequence (`KismetStringLibrary.Conv_StringToName` (`KismetStringLibrary.Concat_StrStr` _returnvalue_2 (`KismetStringLibrary.Conv_NameToString` (`|GetArrayItem` _curvenames 3)))) Time (.roll (.rotation Transform)))
  (`AnimationBlueprintLibrary.AddFloatCurveKey` Sequence (`KismetStringLibrary.Conv_StringToName` (`KismetStringLibrary.Concat_StrStr` _returnvalue_2 (`KismetStringLibrary.Conv_NameToString` (`|GetArrayItem` _curvenames 4)))) Time (.pitch (.rotation Transform)))
  (`AnimationBlueprintLibrary.AddFloatCurveKey` Sequence (`KismetStringLibrary.Conv_StringToName` (`KismetStringLibrary.Concat_StrStr` _returnvalue_2 (`KismetStringLibrary.Conv_NameToString` (`|GetArrayItem` _curvenames 5)))) Time (.yaw (.rotation Transform))))