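; Animation notify that spawns a Niagara shell-casing effect at a configurable socket on the animated mesh.
; When the owner is a Character, it passes the effect its control-rotation forward vector, owner velocity converted into socket space, and a random rotation velocity.
; It also passes velocity bounds, mesh forward axis and casing mesh from ParticleSettings, so one Niagara system can serve different casings.
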(fn `GetNotifyName`
  (returns (ReturnValue :type String))
  (return "Spawn Casing"))

(fn `Received_Notify`
  (params (MeshComp :type "SkeletalMeshComponent Object Reference") (Animation :type "AnimSequenceBase Object Reference") (EventReference :type "AnimNotifyEventReference Structure (by ref)"))
  (returns (ReturnValue :type Boolean))
  (locals (NiagaraComponent :type "NiagaraComponent Object Reference"))
  (bind _particlesettings (`self.ParticleSettings`))
  (bind (_returnvalue_location _returnvalue_rotation) (`KismetMathLibrary.BreakTransform` (`SceneComponent.GetSocketTransform` MeshComp (`self.Socket`) "RTS_World")))
  (bind (_minrotationvelocity_x _minrotationvelocity_y _minrotationvelocity_z) (`KismetMathLibrary.BreakVector` (`/Game/FPSAnimationPack/VFX/BP_CasingParticleSettings.MinRotationVelocity` _particlesettings)))
  (bind (_maxrotationvelocity_x _maxrotationvelocity_y _maxrotationvelocity_z) (`KismetMathLibrary.BreakVector` (`/Game/FPSAnimationPack/VFX/BP_CasingParticleSettings.MaxRotationVelocity` _particlesettings)))
  (bind _returnvalue (`NiagaraFunctionLibrary.SpawnSystemAtLocation` (`/Game/FPSAnimationPack/VFX/BP_CasingParticleSettings.NiagaraSystem` (`self.ParticleSettings`)) _returnvalue_location _returnvalue_rotation))
  (set `local.NiagaraComponent` _returnvalue)
  (bind _ascharacter (cast `Character` (`ActorComponent.GetOwner` (`local.MeshComp`)))
    (:`then`
      (`NiagaraComponent.SetVariableVec3` (`local.NiagaraComponent`) "User.OrientationVector" (`KismetMathLibrary.GetForwardVector` (`Pawn.GetControlRotation` _ascharacter)))
      (`NiagaraComponent.SetVariableVec3` (`local.NiagaraComponent`) "User.MeshForwardAxis" (`/Game/FPSAnimationPack/VFX/BP_CasingParticleSettings.MeshForwardAxis` (`self.ParticleSettings`)))
      (`NiagaraComponent.SetVariableVec3` (`local.NiagaraComponent`) "User.CharacterVelocity" (`KismetMathLibrary.InverseTransformDirection` (`SceneComponent.GetSocketTransform` (`local.MeshComp`) (`self.Socket`) "RTS_World") (`Actor.GetVelocity` (`ActorComponent.GetOwner` (`local.MeshComp`)))))
      (`NiagaraComponent.SetVariableVec3` (`local.NiagaraComponent`) "User.RotationVelocity" (`KismetMathLibrary.MakeVector` (`KismetMathLibrary.RandomFloatInRange` _minrotationvelocity_x _maxrotationvelocity_x) (`KismetMathLibrary.RandomFloatInRange` _minrotationvelocity_y _maxrotationvelocity_y) (`KismetMathLibrary.RandomFloatInRange` _minrotationvelocity_z _maxrotationvelocity_z)))
      (`NiagaraComponent.SetVariableVec3` (`local.NiagaraComponent`) "User.MaxVelocity" (`/Game/FPSAnimationPack/VFX/BP_CasingParticleSettings.MaxVelocity` (`self.ParticleSettings`)))
      (`NiagaraComponent.SetVariableVec3` (`local.NiagaraComponent`) "User.MinVelocity" (`/Game/FPSAnimationPack/VFX/BP_CasingParticleSettings.MinVelocity` (`self.ParticleSettings`)))
      (`NiagaraComponent.SetVariableStaticMesh` (`local.NiagaraComponent`) "User.CasingMesh" (`/Game/FPSAnimationPack/VFX/BP_CasingParticleSettings.CasingMesh` (`self.ParticleSettings`)))
      (return true))
    (:`CastFailed`
      (return true))))