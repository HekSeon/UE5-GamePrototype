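; ViewmodelController is a component on a Character that drives procedural IK motions and holds the active weapon viewmodel settings.
; PlayIKMotion caches the current IKMotion transform, then Tick evaluates the motion over time, blending from that cached transform over the motion's blend time.
; OnViewmodelChanged stores weapon settings and selects their UE4 or UE5 variant.
; ToggleUnrealVersion flips that variant, swapping the Manny mesh and anim class before refreshing the settings.
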(event `self.ReceiveBeginPlay`
  (bind _ascharacter (cast `Character` (`self.GetOwner`)))
  (set `self.Owner Character` _ascharacter))

(event `self.ReceiveTick`
  (params (DeltaSeconds :type "Float (single-precision)"))
  (if (`self.bPlayingIKMotion`)
    (bind _activeikmotion (`self.ActiveIKMotion`)
      (:`then`
        (bind _output_get (set `self.IKMotionPlayback` (+ (* (`/Game/FPSAnimationPack/Blueprints/Procedural/IKMotion.PlayRate` _activeikmotion) DeltaSeconds) (`self.IKMotionPlayback`))))
        (bind _motion (`/Game/FPSAnimationPack/Blueprints/Procedural/IKMotion.Evaluate` (`self.ActiveIKMotion`) _output_get))
        (set `self.IKMotion` (`KismetMathLibrary.TLerp` (`self.CachedIKMotion`) _motion (`KismetMathLibrary.SelectFloat` 1.0 (`KismetMathLibrary.FClamp` (/ (`self.IKMotionPlayback`) (`/Game/FPSAnimationPack/Blueprints/Procedural/IKMotion.BlendTime` (`self.ActiveIKMotion`)))) (`KismetMathLibrary.NearlyEqual_FloatFloat` (`/Game/FPSAnimationPack/Blueprints/Procedural/IKMotion.BlendTime` (`self.ActiveIKMotion`))))))
        (if (>= (`self.IKMotionPlayback`) (`/Game/FPSAnimationPack/Blueprints/Procedural/IKMotion.GetLength` (`self.ActiveIKMotion`)))
          (set `self.bPlayingIKMotion` false)))
      (:`else`))))

(fn `OnViewmodelChanged`
  (params (NewSettings :type "/Game/FPSAnimationPack/Blueprints/Character/WeaponSettings Object Reference"))
  (bind _weaponsettings (`self.WeaponSettings`))
  (set `self.WeaponSettings` NewSettings)
  (set `self.ActiveSettings` (select `bool` (`self.bUE4`) :`false` (`/Game/FPSAnimationPack/Blueprints/Character/WeaponSettings.UE5` _weaponsettings) :`true` (`/Game/FPSAnimationPack/Blueprints/Character/WeaponSettings.UE4` _weaponsettings))))

(fn `PlayIKMotion`
  (params (Motion :type "/Game/FPSAnimationPack/Blueprints/Procedural/IKMotion Object Reference"))
  (set `self.ActiveIKMotion` Motion)
  (set `self.CachedIKMotion` (`self.IKMotion`))
  (set `self.IKMotionPlayback` 0.0)
  (set `self.bPlayingIKMotion` true))

(fn `ToggleUnrealVersion`
  (bind _charactersettings (`self.CharacterSettings`))
  (bind _mesh (`Character.Mesh` (`self.Owner Character`)))
  (bind (_returnvalue_mesh _returnvalue_animblueprint) (break `/Game/FPSAnimationPack/Blueprints/Character/F_CharacterModel` (select `bool` (`self.bUE4`) :`false` (`/Game/FPSAnimationPack/Blueprints/Character/CharacterSettings.MannyUE5` _charactersettings) :`true` (`/Game/FPSAnimationPack/Blueprints/Character/CharacterSettings.MannyUE4` _charactersettings))))
  (set `self.bUE4` (not (`self.bUE4`)))
  (`SkeletalMeshComponent.SetAnimInstanceClass` _mesh _returnvalue_animblueprint)
  (`SkinnedMeshComponent.SetSkinnedAssetAndUpdate` _mesh _returnvalue_mesh true)
  (`self.OnViewmodelChanged` (`self.WeaponSettings`)))