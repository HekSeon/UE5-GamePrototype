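; Weapon manager component for the viewmodel character that spawns its weapons and handles switching between them.
; InitializeWeapons applies the character mesh and AnimBlueprint, then spawns and initializes one weapon actor per settings entry.
; ChangeWeapon sequences unequip and equip montages with delays, hiding the weapon mesh while cycling forward with wraparound.
; OnWeaponChanged swaps the shared weapon mesh and anim class, then syncs aim point and settings with the ViewmodelController.
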(event `ChangeWeapon`
  (bind (_characteranims_primaryreload _characteranims_secondaryreload _characteranims_additionalreload _characteranims_equip) (break `/Game/FPSAnimationPack/Blueprints/Character/F_ViewmodelAnimations` (`/Game/FPSAnimationPack/Blueprints/Character/ViewmodelSettings.CharacterAnims` (`/Game/FPSAnimationPack/Blueprints/Weapon/BP_WeaponBase.ViewmodelSettings` (`self.ActiveWeapon`)))))
  (bind (_characteranims_primaryreload_2 _characteranims_secondaryreload_2 _characteranims_additionalreload_2 _characteranims_equip_2 _characteranims_unequip) (break `/Game/FPSAnimationPack/Blueprints/Character/F_ViewmodelAnimations` (`/Game/FPSAnimationPack/Blueprints/Character/ViewmodelSettings.CharacterAnims` (`/Game/FPSAnimationPack/Blueprints/Weapon/BP_WeaponBase.ViewmodelSettings` (`self.ActiveWeapon`)))))
  (bind (_weaponanims_primaryreload _weaponanims_secondaryreload _weaponanims_additionalreload _weaponanims_equip) (break `/Game/FPSAnimationPack/Blueprints/Character/F_ViewmodelAnimations` (`/Game/FPSAnimationPack/Blueprints/Character/WeaponSettings.WeaponAnims` (`/Game/FPSAnimationPack/Blueprints/Weapon/BP_WeaponBase.WeaponSettings` (`self.ActiveWeapon`)))))
  (`|PlayMontage` (`Character.Mesh` (`self.Owner Character`)) _characteranims_unequip
    (:`then`
      (`KismetSystemLibrary.Delay` (`AnimSequenceBase.SequenceLength` _characteranims_unequip))
      (`SceneComponent.SetVisibility` (`/Game/FPSAnimationPack/Blueprints/Character/BP_ViewmodelCharacter.WeaponMesh` (`self.Owner Character`)) false true)
      (`/Game/FPSAnimationPack/Blueprints/Weapon/BP_WeaponBase.OnUnEquipped` (`self.ActiveWeapon`))
      (`self.CycleWeapons` true)
      (`|PlayMontage` (`Character.Mesh` (`self.Owner Character`)) _characteranims_equip
        (:`then`
          (`|PlayMontage` (`/Game/FPSAnimationPack/Blueprints/Character/BP_ViewmodelCharacter.WeaponMesh` (`self.Owner Character`)) _weaponanims_equip
            (:`then`
              (`self.OnWeaponChanged`)
              (`KismetSystemLibrary.Delay` 0.05)
              (`SceneComponent.SetVisibility` (`/Game/FPSAnimationPack/Blueprints/Character/BP_ViewmodelCharacter.WeaponMesh` (`self.Owner Character`)) true true))))))))

(event `self.ReceiveTick`
  (params (DeltaSeconds :type "Float (single-precision)")))

(fn `CycleWeapons`
  (params (Forward :type Boolean))
  (bind _returnvalue (+ (`self.ActiveWeaponIndex`) 1))
  (bind _returnvalue_2 (- (`self.ActiveWeaponIndex`) 1))
  (bind _returnvalue_3 (- (`KismetArrayLibrary.Array_Length` (`self.Weapons`)) 1))
  (if Forward
    (set `self.ActiveWeaponIndex` (`KismetMathLibrary.SelectInt` 0 _returnvalue (> _returnvalue _returnvalue_3)))
    (else
      (set `self.ActiveWeaponIndex` (`KismetMathLibrary.SelectInt` _returnvalue_3 _returnvalue_2 (< _returnvalue_2 0)))))
  (`self.OnWeaponChanged`))

(fn `InitializeWeapons`
  (params (CharSettings :type "/Game/FPSAnimationPack/Blueprints/Character/CharacterSettings Object Reference"))
  (bind _owner_character (`self.Owner Character`))
  (bind (_mesh _animblueprint) (break `/Game/FPSAnimationPack/Blueprints/Character/F_CharacterModel` (`/Game/FPSAnimationPack/Blueprints/Character/CharacterSettings.MannyUE4` (`local.CharSettings`))))
  (set `self.ViewmodelComponent` (`Actor.GetComponentByClass` (`self.GetOwner`) "/Game/FPSAnimationPack/Blueprints/Character/ViewmodelController.ViewmodelController_C"))
  (bind _asbp_viewmodel_character (cast `/Game/FPSAnimationPack/Blueprints/Character/BP_ViewmodelCharacter` (`self.GetOwner`)))
  (bind _output_get (set `self.Owner Character` _asbp_viewmodel_character))
  (bind _mesh_2 (`Character.Mesh` _output_get))
  (`SkeletalMeshComponent.SetAnimInstanceClass` _mesh_2 _animblueprint)
  (`SkinnedMeshComponent.SetSkinnedAssetAndUpdate` _mesh_2 _mesh true)
  (for _array_element (`/Game/FPSAnimationPack/Blueprints/Character/CharacterSettings.Settings` (`local.CharSettings`))
    (bind _returnvalue (`|SpawnActorFromClass` (`/Game/FPSAnimationPack/Blueprints/Character/WeaponSettings.WeaponClass` _array_element) (`Actor.GetTransform` _owner_character) "Undefined" "SelectDefaultAtRuntime" _owner_character null))
    (`/Game/FPSAnimationPack/Blueprints/Weapon/BP_WeaponBase.Initialize` _returnvalue _array_element)
    (`KismetArrayLibrary.Array_Add` (`self.Weapons`) _returnvalue))
  (set `self.ActiveWeapon` (`|GetArrayItem` (`self.Weapons`)))
  (`self.OnWeaponChanged`))

(fn `OnWeaponChanged`
  (bind _weaponsettings (`/Game/FPSAnimationPack/Blueprints/Weapon/BP_WeaponBase.WeaponSettings` (`self.ActiveWeapon`)))
  (`/Game/FPSAnimationPack/Blueprints/Weapon/BP_WeaponBase.OnUnEquipped` (`self.ActiveWeapon`))
  (set `self.ActiveWeapon` (`|GetArrayItem` (`self.Weapons`) (`self.ActiveWeaponIndex`)))
  (`SkinnedMeshComponent.SetSkinnedAssetAndUpdate` (`/Game/FPSAnimationPack/Blueprints/Character/BP_ViewmodelCharacter.WeaponMesh` (`self.Owner Character`)) (`/Game/FPSAnimationPack/Blueprints/Character/WeaponSettings.WeaponMesh` _weaponsettings) true)
  (`SkeletalMeshComponent.SetAnimInstanceClass` (`/Game/FPSAnimationPack/Blueprints/Character/BP_ViewmodelCharacter.WeaponMesh` (`self.Owner Character`)) (`/Game/FPSAnimationPack/Blueprints/Character/WeaponSettings.WeaponAnimInstance` _weaponsettings))
  (`/Game/FPSAnimationPack/Blueprints/Weapon/BP_WeaponBase.OnEquipped` (`self.ActiveWeapon`))
  (bind _viewmodelcomponent (`self.ViewmodelComponent`)
    (:`then`
      (`/Game/FPSAnimationPack/Blueprints/Character/ViewmodelController.OnViewmodelChanged` _viewmodelcomponent (`/Game/FPSAnimationPack/Blueprints/Weapon/BP_WeaponBase.WeaponSettings` (`self.ActiveWeapon`)))
      (set `/Game/FPSAnimationPack/Blueprints/Character/ViewmodelController.ActiveAimPoint` (`/Game/FPSAnimationPack/Blueprints/Weapon/BP_WeaponBase.AimPoint` (`self.ActiveWeapon`)) (`self.ViewmodelComponent`))
      (`self.RefreshWeaponSettings`))
    (:`else`)))

(fn `RefreshWeaponSettings`
  (set `/Game/FPSAnimationPack/Blueprints/Weapon/BP_WeaponBase.ViewmodelSettings` (`/Game/FPSAnimationPack/Blueprints/Character/ViewmodelController.ActiveSettings` (`self.ViewmodelComponent`)) (`self.ActiveWeapon`)))