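; Player character for the FPS animation pack that turns Enhanced Input into movement, look, weapon and viewmodel actions.
; Weapon input raises calls like fire and reload, or drives WeaponManager, which initializes from ViewmodelController's character settings.
; Sprint inputs set a movement state that Tick turns into animation gait and interpolated walk speed.
; Aiming, allowed only outside sprint, updates ViewmodelController and RecoilAnimation with sound and IK motion.
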(event `self.ReceivePossessed`
  (params (NewController :type "Controller Object Reference"))
  (bind _asplayer_controller (cast `PlayerController` NewController))
  (`EnhancedInputSubsystemInterface.AddMappingContext` (pcsubsystem `EnhancedInputLocalPlayerSubsystem` _asplayer_controller) "/Game/FPSAnimationPack/Input/IMC_FPSAnimation.IMC_FPSAnimation" 0 (struct)))

(event `self.ReceiveBeginPlay`
  (`/Game/FPSAnimationPack/Blueprints/Character/WeaponManager.InitializeWeapons` (`self.WeaponManager`) (`/Game/FPSAnimationPack/Blueprints/Character/ViewmodelController.CharacterSettings` (`self.ViewmodelController`))))

(event `self.ReceiveTick`
  (params (DeltaSeconds :type "Float (single-precision)"))
  (`self.UpdateMovement` DeltaSeconds))

(event `EnhancedInput|/Game/FPSAnimationPack/Input/IA_Pickup`
  (params (ActionValue :type Boolean) (ElapsedSeconds :type "Float (double-precision)") (TriggeredSeconds :type "Float (double-precision)") (InputAction :type "InputAction Object Reference" :default "/Game/FPSAnimationPack/Input/IA_Pickup.IA_Pickup"))
  ;[0 0 0] Weapon Actions
  (:`Triggered`
    (`self.OnInteractPressed`)))

(event `EnhancedInput|/Game/FPSAnimationPack/Input/IA_Reload`
  (params (ActionValue :type Boolean) (ElapsedSeconds :type "Float (double-precision)") (TriggeredSeconds :type "Float (double-precision)") (InputAction :type "InputAction Object Reference" :default "/Game/FPSAnimationPack/Input/IA_Reload.IA_Reload"))
  ;[0 0 0] Weapon Actions
  (:`Triggered`
    (`self.OnReloadPressed`)))

(event `EnhancedInput|/Game/FPSAnimationPack/Input/IA_Move`
  (params (ActionValue :type "Vector2D Structure") (ElapsedSeconds :type "Float (double-precision)") (TriggeredSeconds :type "Float (double-precision)") (InputAction :type "InputAction Object Reference" :default "/Game/FPSAnimationPack/Input/IA_Move.IA_Move"))
  ;[0 0 0] Input Actions
  (:`Triggered`
    (`self.AddMovementInput` (`self.GetActorRightVector`) ActionValue_X)
    (`self.AddMovementInput` (`self.GetActorForwardVector`) ActionValue_Y)
    (set `self.MoveInput` (`KismetMathLibrary.MakeVector2D` ActionValue_X ActionValue_Y))))

(event `EnhancedInput|/Game/FPSAnimationPack/Input/IA_Look`
  (params (ActionValue :type "Vector2D Structure") (ElapsedSeconds :type "Float (double-precision)") (TriggeredSeconds :type "Float (double-precision)") (InputAction :type "InputAction Object Reference" :default "/Game/FPSAnimationPack/Input/IA_Look.IA_Look"))
  ;[0 0 0] Input Actions
  (:`Triggered`
    (`self.AddControllerYawInput` ActionValue_X)
    (`self.AddControllerPitchInput` ActionValue_Y)))

(event `EnhancedInput|/Game/FPSAnimationPack/Input/IA_Aim`
  (params (ActionValue :type Boolean) (ElapsedSeconds :type "Float (double-precision)") (TriggeredSeconds :type "Float (double-precision)") (InputAction :type "InputAction Object Reference" :default "/Game/FPSAnimationPack/Input/IA_Aim.IA_Aim"))
  (bind _returnvalue (`|EnumEquality` (`self.MovementState`) "NewEnumerator5"))
  ;[0 0 0] Weapon Actions
  (:`Triggered`
    (if ActionValue
      (if _returnvalue
        (`self.SetAiming` true)
        (`/Game/FPSAnimationPack/Blueprints/Character/ViewmodelController.PlayIKMotion` (`self.ViewmodelController`) "/Game/FPSAnimationPack/Blueprints/Procedural/Ads/IK_Ads.IK_Ads" :!label _label))
      (elif _returnvalue
        (`self.SetAiming` false)
        (goto _label)))))

(event `EnhancedInput|/Game/FPSAnimationPack/Input/IA_Grenade`
  (params (ActionValue :type Boolean) (ElapsedSeconds :type "Float (double-precision)") (TriggeredSeconds :type "Float (double-precision)") (InputAction :type "InputAction Object Reference" :default "/Game/FPSAnimationPack/Input/IA_Grenade.IA_Grenade"))
  ;[0 0 0] Weapon Actions
  (:`Triggered`
    (`self.OnGrenade`)))

(event `EnhancedInput|/Game/FPSAnimationPack/Input/IA_Version`
  (params (ActionValue :type Boolean) (ElapsedSeconds :type "Float (double-precision)") (TriggeredSeconds :type "Float (double-precision)") (InputAction :type "InputAction Object Reference" :default "/Game/FPSAnimationPack/Input/IA_Version.IA_Version"))
  ;[0 0 0] Weapon Actions
  (:`Triggered`
    (`/Game/FPSAnimationPack/Blueprints/Character/ViewmodelController.ToggleUnrealVersion` (`self.ViewmodelController`))
    (`/Game/FPSAnimationPack/Blueprints/Character/WeaponManager.RefreshWeaponSettings` (`self.WeaponManager`))))

(event `EnhancedInput|/Game/FPSAnimationPack/Input/IA_Sprint`
  (params (ActionValue :type Boolean) (ElapsedSeconds :type "Float (double-precision)") (TriggeredSeconds :type "Float (double-precision)") (InputAction :type "InputAction Object Reference" :default "/Game/FPSAnimationPack/Input/IA_Sprint.IA_Sprint"))
  ;[0 0 0] Input Actions
  (:`Triggered`
    (if ActionValue
      (set `self.MovementState` "NewEnumerator6")
      (`self.SetAiming` false)
      (else
        (set `self.MovementState` "NewEnumerator5")))))

(event `EnhancedInput|/Game/FPSAnimationPack/Input/IA_ChangeWeapon`
  (params (ActionValue :type Boolean) (ElapsedSeconds :type "Float (double-precision)") (TriggeredSeconds :type "Float (double-precision)") (InputAction :type "InputAction Object Reference" :default "/Game/FPSAnimationPack/Input/IA_ChangeWeapon.IA_ChangeWeapon"))
  ;[0 0 0] Weapon Actions
  (:`Triggered`
    (`/Game/FPSAnimationPack/Blueprints/Character/WeaponManager.ChangeWeapon` (`self.WeaponManager`))))

(event `EnhancedInput|/Game/FPSAnimationPack/Input/IA_Firemode`
  (params (ActionValue :type Boolean) (ElapsedSeconds :type "Float (double-precision)") (TriggeredSeconds :type "Float (double-precision)") (InputAction :type "InputAction Object Reference" :default "/Game/FPSAnimationPack/Input/IA_Firemode.IA_Firemode"))
  ;[0 0 0] Weapon Actions
  (:`Triggered`
    (`self.OnFireMode`)))

(event `EnhancedInput|/Game/FPSAnimationPack/Input/IA_TacSprint`
  (params (ActionValue :type Boolean) (ElapsedSeconds :type "Float (double-precision)") (TriggeredSeconds :type "Float (double-precision)") (InputAction :type "InputAction Object Reference" :default "/Game/FPSAnimationPack/Input/IA_TacSprint.IA_TacSprint"))
  (bind _movementstate (`self.MovementState`))
  ;[0 0 0] Input Actions
  (:`Triggered`
    (if ActionValue
      (if (`|EnumEquality` _movementstate "NewEnumerator6")
        (set `self.MovementState` "NewEnumerator7"))
      (elif (`|EnumEquality` _movementstate "NewEnumerator7")
        (set `self.MovementState` "NewEnumerator6")))))

(event `EnhancedInput|/Game/FPSAnimationPack/Input/IA_Fire`
  (params (ActionValue :type Boolean) (ElapsedSeconds :type "Float (double-precision)") (TriggeredSeconds :type "Float (double-precision)") (InputAction :type "InputAction Object Reference" :default "/Game/FPSAnimationPack/Input/IA_Fire.IA_Fire"))
  ;[0 0 0] Weapon Actions
  (:`Triggered`
    (bind _output_get (set `/Game/FPSAnimationPack/Blueprints/Character/ViewmodelController.IsPressingTrigger` ActionValue (`self.ViewmodelController`)))
    (if _output_get
      (`self.OnFirePressed`)
      (else
        (`self.OnFireReleased`)))))

(event `EnhancedInput|/Game/FPSAnimationPack/Input/IA_CycleViewmodel`
  (params (ActionValue :type "Float (double-precision)") (ElapsedSeconds :type "Float (double-precision)") (TriggeredSeconds :type "Float (double-precision)") (InputAction :type "InputAction Object Reference" :default "/Game/FPSAnimationPack/Input/IA_CycleViewmodel.IA_CycleViewmodel"))
  (bind _weaponmanager (`self.WeaponManager`))
  ;[0 0 0] Weapon Actions
  (:`Triggered`
    (if (> ActionValue 0.0)
      (`/Game/FPSAnimationPack/Blueprints/Character/WeaponManager.CycleWeapons` _weaponmanager true)
      (else
        (`/Game/FPSAnimationPack/Blueprints/Character/WeaponManager.CycleWeapons` _weaponmanager false)))))

(event `EnhancedInput|/Game/FPSAnimationPack/Input/IA_Jump`
  (params (ActionValue :type Boolean) (ElapsedSeconds :type "Float (double-precision)") (TriggeredSeconds :type "Float (double-precision)") (InputAction :type "InputAction Object Reference" :default "/Game/FPSAnimationPack/Input/IA_Jump.IA_Jump"))
  ;[0 0 0] Input Actions
  (:`Triggered`
    (`self.Jump`)))

(event `EnhancedInput|/Game/FPSAnimationPack/Input/IA_Inspect`
  (params (ActionValue :type Boolean) (ElapsedSeconds :type "Float (double-precision)") (TriggeredSeconds :type "Float (double-precision)") (InputAction :type "InputAction Object Reference" :default "/Game/FPSAnimationPack/Input/IA_Inspect.IA_Inspect"))
  ;[0 0 0] Weapon Actions
  (:`Triggered`
    (`self.PlayAnimMontage` "/Game/FPSAnimationPack/Animations/UE4/General/Character/AM_FP_Inspect.AM_FP_Inspect")))

(event `EnhancedInput|/Game/Input/IA_Interact`
  (params (ActionValue :type Boolean) (ElapsedSeconds :type "Float (double-precision)") (TriggeredSeconds :type "Float (double-precision)") (InputAction :type "InputAction Object Reference" :default "/Game/Input/IA_Interact.IA_Interact")))

(fn `SetAiming`
  (params (IsAiming :type Boolean))
  (if (!= IsAiming (`/Game/FPSAnimationPack/Blueprints/Character/ViewmodelController.IsAiming` (`self.ViewmodelController`)))
    (set `/Game/FPSAnimationPack/Blueprints/Character/ViewmodelController.IsAiming` IsAiming (`self.ViewmodelController`))
    (`RecoilAnimationComponent.SetAimingStatus` (`self.RecoilAnimation`) (`local.IsAiming`))
    (if (`local.IsAiming`)
      (`GameplayStatics.PlaySound2D` "/Game/FPSAnimationPack/SFX/General/S_Aim_In.S_Aim_In" 1.0 1.0 0.0 null null)
      (else
        (`GameplayStatics.PlaySound2D` "/Game/FPSAnimationPack/SFX/General/S_Aim_Out.S_Aim_Out" 1.0 1.0 0.0 null null)))))

(fn `UpdateMovement`
  (params (DeltaTime :type "Float (double-precision)"))
  (set `/Game/FPSAnimationPack/Blueprints/Character/ViewmodelController.Gait` (`KismetMathLibrary.SelectFloat` (`KismetMathLibrary.FClamp` (`KismetMathLibrary.VSize2D` (`self.MoveInput`))) (`KismetMathLibrary.SelectFloat` 3.0 2.0 (`|EnumEquality` (`self.MovementState`) "NewEnumerator7")) (`|EnumEquality` (`self.MovementState`) "NewEnumerator5")) (`self.ViewmodelController`))
  (set `self.DesiredSpeed` (`KismetMathLibrary.SelectFloat` 250.0 (`KismetMathLibrary.SelectFloat` 500.0 400.0 (`|EnumEquality` (`self.MovementState`) "NewEnumerator7")) (`|EnumEquality` (`self.MovementState`) "NewEnumerator5")))
  (bind _output_get (set `self.Speed` (`KismetMathLibrary.FInterpTo` (`self.Speed`) (`self.DesiredSpeed`) DeltaTime)))
  (set `CharacterMovementComponent.MaxWalkSpeed` _output_get (`self.CharacterMovement`)))

(fn `UserConstructionScript`)